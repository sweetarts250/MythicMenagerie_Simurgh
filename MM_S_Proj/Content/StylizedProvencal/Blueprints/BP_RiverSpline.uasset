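; BP_RiverSpline is a spline-driven actor for laying out a river, built in the construction script.
; It adds one spline mesh component per segment, storing each in the Mesh array and bending it between neighboring points using local positions and tangents.
; A second pass loops over those meshes but does nothing, as the water material assignment is disconnected.
; The event graph has no active logic.
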(fn `UserConstructionScript`
  (bind _spline (`self.Spline`))
  (`|ExecutionSequence`
    (:`then_0`
      (for _index (range (+ (- (`SplineComponent.GetNumberOfSplinePoints` _spline) 2) 1))
        (bind _returnvalue (`AddComponent|NODE_AddSplineMeshComponent-1`))
        (`KismetArrayLibrary.Array_Add` (`self.Mesh`) _returnvalue)
        (`self.K2_AttachToComponent` (`self.DefaultSceneRoot`) "None" "KeepRelative" "KeepRelative" "KeepRelative")
        (bind (_location _tangent) (`SplineComponent.GetLocationAndTangentAtSplinePoint` _spline _index "Local"))
        (bind (_location_2 _tangent_2) (`SplineComponent.GetLocationAndTangentAtSplinePoint` _spline (+ _index 1) "Local"))
        (`SplineMeshComponent.SetStartAndEnd` _returnvalue _location _tangent _location_2 _tangent_2 true)))
    (:`then_1`
      (for _array_element (`self.Mesh`)
        _))))